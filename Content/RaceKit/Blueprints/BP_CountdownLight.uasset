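; BP_CountdownLight is a RaceKit countdown light that flashes on race countdown ticks and turns green at zero.
; It creates a dynamic material on its mesh and binds to the countdown event of the manager for its RaceID.
; Each tick restarts the ReduceBrightness timeline to fade emissive brightness, with the default red color replaced by green on the final tick.
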(event `self.ReceiveBeginPlay`
  (bind _returnvalue (`PrimitiveComponent.CreateDynamicMaterialInstance` (`self.StaticMesh`) 0 null))
  (set `self.LightMID` _returnvalue)
  (bind _racekitmanager (`/Game/RaceKit/Blueprints/BPFL_RaceKitFunctions.GetRaceKitManager` (`self.RaceID`)))
  (`/Engine/EditorBlueprintResources/StandardMacros.IsValid` _racekitmanager
    (:`Is Valid`
      (add `/Game/RaceKit/Blueprints/BP_RaceKitManager.RaceCountDown` _racekitmanager (delegate `RaceCountDown`)))))

(event `RaceCountDown`
  (params (TimeLeft :type Integer))
  ;[1 1 1] On zero, instead of default red emissive color, use green.
  (if (== TimeLeft 0)
    (`MaterialInstanceDynamic.SetVectorParameterValue` (`self.LightMID`) "EmissiveColor" (struct :`G` 1.0 :`A` 1.0))
    ;[1 1 1] Fade emissive brightness
    (bind (_direction _brightness) (`Timeline|ReduceBrightness` :!via `PlayFromStart` :!label _label)
      (:`Update`
        (`MaterialInstanceDynamic.SetScalarParameterValue` (`self.LightMID`) "EmissiveAmount" _brightness)))
    (else
      (goto _label :!via `PlayFromStart`))))

(fn `LightCountdown`
  (params (Timeleft :type Integer) (Timeline :type "TimelineComponent Object Reference")))

(fn `UserConstructionScript`)