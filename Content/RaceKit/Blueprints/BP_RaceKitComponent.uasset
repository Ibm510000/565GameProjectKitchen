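; Racer component that tracks one actor's lap, next checkpoint, lap times and finish in a race.
; It registers with the RaceKitManager for its RaceID, which supplies checkpoints and decides finishes when a checkpoint is hit.
; While racing, Tick accumulates lap time and updates a dot-product distance to the next checkpoint.
; CompareTo orders racers by lap, checkpoint (with a zero-index special case), then distance, returning -1 for ahead.
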(event EventBeginPlay
  ;[1 1 1] Call to setup variables before starting each race.
  (CallFunction|SetupforRace))

(event EventTick
  (params (DeltaSeconds :type Float%20%28single-precision%29))
  ;[1 1 1] If racing, calculate positional data and count current lap time.
  (if (Variables|Data|GetRacing)
    (Utilities|FlowControl|Sequence
      (:then_0
        (CallFunction|SetNextCheckPointDistance))
      (:then_1
        (CallFunction|CountLapTime)))))

(fn HitCheckPoint
  (params (HitCheckPoint :type Integer))
  ;[1 1 1] Tell manager which check point was hit to check if finished based on Race Mode.
  (bind _finished (Default|CompareCheckPoint (Variables|Data|GetRaceKitManager) HitCheckPoint (Variables|Data|GetNextCheckPoint) (Variables|Data|GetLap)))
  (if _finished
    ;[1 1 1] Hit the finish, compare if best lap time and notifiy manager for placement.
    (CallFunction|CheckBestLapTime true)
    (Variables|Data|SetRacing false)
    (Default|FinishedRacer (Variables|Data|GetRaceKitManager) (Variables|Data|GetRacerSlot))
    (else
      ;[1 1 1] Get Next Check Point from Manager, set data, and if next lap increment lap and compare best lap time.
      (bind (_racekitcheckpoint _nextcheckpoint _nextlap) (Default|GetCheckPoint (Variables|Data|GetRaceKitManager) HitCheckPoint (Variables|Data|GetNextCheckPoint)))
      (Variables|Data|SetRaceKitCheckPointActor _racekitcheckpoint)
      (Variables|Data|SetNextCheckPoint _nextcheckpoint)
      (CallFunction|SetNextCheckPointDistance)
      (if _nextlap
        (Math|Integer|IncrementInt (Variables|Data|GetLap)
          (:%20%20
            (CallFunction|CheckBestLapTime false)))))))

(fn GetData
  ;[1 1 1] Returns all positional race data of this racer.
  (return (Variables|Data|GetNextCheckPointDistance) (Variables|Data|GetNextCheckPoint) (Variables|Data|GetLap)))

(fn SetNextCheckPointDistance
  (bind _racerfront (CallFunction|GetRacerFront))
  (bind (_checkpointfront _checkpointheading) (CallFunction|GetNextCheckPointData))
  ;[1 1 1] Based on the racer position and the checkpoint position, calculate an accurate float distance to the next checkpoint.
  (bind _output_get (Variables|Data|SetNextCheckPointDistance (Math|Vector|DotProduct (- _racerfront _checkpointfront) (- _racerfront _checkpointheading))))
  (return _output_get))

(fn GetRacerFront
  ;[1 1 1] Return the world space vector of the front of the racer.
  (return (Math|Transform|TransformLocation (Transformation|GetActorTransform (Components|GetOwner)) (Variables|Settings|GetFront))))

(fn GetNextCheckPointData
  (bind _racekitcheckpointactor (Variables|Data|GetRaceKitCheckPointActor))
  ;[1 1 1] Get desired checkpoint's positional data.
  (return (Default|GetCheckPointFront _racekitcheckpointactor) (Math|Transform|TransformLocation (Transformation|GetActorTransform _racekitcheckpointactor) (Variables|/Game/RaceKit/Blueprints/BP_RaceKitCheckPoint.BP_RaceKitCheckPoint_C|GetHeading _racekitcheckpointactor))))

(fn CheckBestLapTime
  (params (Finished :type Boolean))
  ;[1 1 1] The lap time will need to be set to 0 on a new lap if the race isn't finished, or can be left as the current lap time if the race is finished.
  (if (Math|Boolean|Equal(Boolean) Finished true)
    (LocalVariables|SetLocalLapTime (Variables|Data|GetLapTime))
    (else
      (LocalVariables|SetLocalLapTime 0.0)))
  ;[1 1 1] If best lap time is 0, the first lap completed is the best time.
  (if (== (Variables|Data|GetBestLapTime) 0.0)
    (Variables|Data|SetBestLapTime (Variables|Data|GetLapTime))
    (Variables|Data|SetLapTime (LocalVariables|GetLocalLapTime))
    (else
      ;[1 1 1] If best lap time is > 0, compare current lap time to best lap time.
      (if (< (Variables|Data|GetLapTime) (Variables|Data|GetBestLapTime))
        (Variables|Data|SetBestLapTime (Variables|Data|GetLapTime))
        (Variables|Data|SetLapTime (LocalVariables|GetLocalLapTime))
        (else
          (Variables|Data|SetLapTime (LocalVariables|GetLocalLapTime))))))
  (return))

(fn SetupforRace
  ;[1 1 1] Store a reference to the desired Manager.
  (bind _racekitmanager (CallFunction|GetRaceKitManager (Variables|Settings|GetRaceID)))
  (bind _output_get (Variables|Data|SetRaceKitManager _racekitmanager))
  ;[1 1 1] Register racer in the manager so the manager can set position.
  (Utilities|IsValid _output_get
    (:Is%20Valid
      (Default|RegisterRacer (Variables|Data|GetRaceKitManager) self)
      ;[1 1 1] Save first desired checkpoint and set initial race positional data.
      (bind _racekitcheckpoint (Default|GetCheckPoint (Variables|Data|GetRaceKitManager) 0 (Variables|Data|GetNextCheckPoint)))
      (Variables|Data|SetRaceKitCheckPointActor _racekitcheckpoint)
      (CallFunction|SetNextCheckPointDistance))
    (:Is%20Not%20Valid
      _))
  (return))

(fn CountLapTime
  ;[1 1 1] Count the time elapsed of the current lap.
  (Variables|Data|SetLapTime (+ (Utilities|Time|GetWorldDeltaSeconds) (Variables|Data|GetLapTime)))
  (return))

(fn ResetRacer
  ;[1 1 1] Clear out and reset race data to prepare for another race.
  (Variables|Data|SetNextCheckPoint 1)
  (Variables|Data|SetFinished false)
  (Variables|Data|SetLapTime 0.0)
  (Variables|Data|SetBestLapTime 0.0)
  (Variables|Data|SetFinishedPosition 0))

(fn Compareto
  (params (Other :type Object%20Object%20Reference))
  (bind (_nextcheckpointdistance _nextcheckpoint _lap) (CallFunction|GetData))
  ;[1 1 1] Comparing components is done by comparing the race data of this component and another component.
  (bind _asbp_race_kit_component (Utilities|Casting|CastToBP_RaceKitComponent Other)
    (:then
      ;[1 1 1] Save local variables of this component's race data and the other component's race data for a clean graph.
      (Utilities|FlowControl|Sequence
        (:then_0
          (LocalVariables|SetLocalNextCheckPointDistance _nextcheckpointdistance))
        (:then_1
          (LocalVariables|SetLocalNextCheckPoint _nextcheckpoint))
        (:then_2
          (LocalVariables|SetLocalLap _lap))
        (:then_3
          (LocalVariables|SetLocalOtherNextCheckPointDistance (.NextCheckPointDistance (CallFunction|GetData _asbp_race_kit_component))))
        (:then_4
          (LocalVariables|SetLocalOtherNextCheckPoint (.NextCheckPoint (CallFunction|GetData _asbp_race_kit_component))))
        (:then_5
          (LocalVariables|SetLocalOtherLap (.Lap (CallFunction|GetData _asbp_race_kit_component))))
        (:then_6
          (Utilities|FlowControl|Sequence
            (:then_0
              ;[1 1 1] Racer is ahead if lap is greater.
              (if (> (LocalVariables|GetLocalLap) (LocalVariables|GetLocalOtherLap))
                (bind _output_get (LocalVariables|SetLocalResult -1))
                (return _output_get)))
            (:then_1
              (if (< (LocalVariables|GetLocalLap) (LocalVariables|GetLocalOtherLap))
                (bind _output_get_2 (LocalVariables|SetLocalResult 1))
                (return _output_get_2)))
            (:then_2
              ;[1 1 1] Racer is ahead if checkpoint is greater, and behind if less, with a special case depending on the 0 checkpoint.
              (if (> (LocalVariables|GetLocalNextCheckPoint) (LocalVariables|GetLocalOtherNextCheckPoint))
                (bind _output_get_3 (LocalVariables|SetLocalResult -1))
                (return _output_get_3)))
            (:then_3
              (if (< (LocalVariables|GetLocalNextCheckPoint) (LocalVariables|GetLocalOtherNextCheckPoint))
                (if (== (LocalVariables|GetLocalNextCheckPoint) 0)
                  (LocalVariables|SetLocalResult -1)
                  (else
                    (LocalVariables|SetLocalResult 1)))
                (return (LocalVariables|GetLocalResult))))
            (:then_4
              ;[1 1 1] If not ahead in laps or checkpoints, compare the checkpoint distance data.
              (if (< (LocalVariables|GetLocalNextCheckPointDistance) (LocalVariables|GetLocalOtherNextCheckPointDistance))
                (bind _output_get_4 (LocalVariables|SetLocalResult -1))
                (return _output_get_4)))
            (:then_5
              (if (> (LocalVariables|GetLocalNextCheckPointDistance) (LocalVariables|GetLocalOtherNextCheckPointDistance))
                (bind _output_get_5 (LocalVariables|SetLocalResult 1))
                (return _output_get_5)))
            (:then_6
              ;[1 1 1] Return the comparison int.
              (return (LocalVariables|GetLocalResult)))))))
    (:CastFailed
      (return 0))))