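; BP_MeshRacer is a racer actor that moves a static mesh around a spline track in timed laps.
; The construction script sets the spline duration to RaceTime, and BeginPlay detaches the spline so the track stays in place.
; While RaceKitComponent is Racing, Tick advances a timer, places and rotates the mesh at that time along the spline, and resets the timer to start a new lap.
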(event `self.ReceiveBeginPlay`
  ;[1 1 1] Detach the Spline so that it stays in one place as the Mesh Racer follows it.
  (`SceneComponent.DetachFromParent` (`self.Spline`) true true))

(event `self.ReceiveTick`
  (params (DeltaSeconds :type "Float (single-precision)"))
  (bind _currenttime (`self.CurrentTime`))
  (bind _spline (`self.Spline`))
  (if (`/Game/RaceKit/Blueprints/BP_RaceKitComponent.Racing` (`self.RaceKitComponent`))
    (`|ExecutionSequence`
      (:`then_0`
        ;[1 1 1] Increment current time along spline, which gives the location on the spline where the Mesh Racer should be.
        (set `self.CurrentTime` (+ (`self.CurrentTime`) (`GameplayStatics.GetWorldDeltaSeconds`)))
        ;[1 1 1] Set mesh location and rotation along spline
        (`SceneComponent.K2_SetWorldLocationAndRotation` (`self.StaticMesh`) (`SplineComponent.GetLocationAtTime` _spline _currenttime "World" false) (`SplineComponent.GetRotationAtTime` _spline _currenttime "World" false) false false))
      (:`then_1`
        ;[1 1 1] Reset time counter when hitting Race Time, which will start a new lap.
        (if (>= (`self.CurrentTime`) (`self.RaceTime`))
          (set `self.CurrentTime` 0.0))))))

(fn `UserConstructionScript`
  ;[1 1 1] Set the amount of time it takes the Mesh Racer to complete one lap
  (set `SplineComponent.Duration` (`self.RaceTime`) (`self.Spline`)))