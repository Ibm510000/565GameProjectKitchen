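; Race checkpoint actor with a numbered box volume that tells an overlapping racer's BP_RaceKitComponent it was hit.
; It then fires a HitCheckPoint dispatcher so levels can react to specific checkpoints.
; The construction script sizes the box, offsets a debug arrow and text from its extent, and shows the number when debug is enabled.
; Helpers compare checkpoints by number and return a front position offset along world X.
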(event `self.ReceiveActorBeginOverlap`
  (params (OtherActor :type "Actor Object Reference"))
  (bind _output (`|GetArrayItem` (`self.K2_GetComponentsByClass` OtherActor "/Game/RaceKit/Blueprints/BP_RaceKitComponent.BP_RaceKitComponent_C")))
  ;[1 1 1] On checkpoint hit, notify the racer's Race Kit Component that a checkpoint has been hit so it can update to the next checkpoint.
  (`/Engine/EditorBlueprintResources/StandardMacros.IsValid` _output
    (:`Is Valid`
      (`/Game/RaceKit/Blueprints/BP_RaceKitComponent.HitCheckPoint` _output (`self.CheckPoint`))
      ;[1 1 1] Add level effects or modifications based on hitting certain checkpoints by getting a reference to the checkpoint and subscribing to this event
      (`self.HitCheckPoint`))))

(fn `CompareTo`
  (params (Other :type "Object Object Reference"))
  (returns (Result :type Integer))
  (locals (LocalResult :type Integer))
  ;[1 1 1] Compare checkpoints by checkpoint number.
  (bind _asbp_race_kit_check_point (cast `/Game/RaceKit/Blueprints/BP_RaceKitCheckPoint` Other)
    (:`then`
      (`/Engine/EditorBlueprintResources/StandardMacros.CompareInt` (`self.CheckPoint`) (`/Game/RaceKit/Blueprints/BP_RaceKitCheckPoint.CheckPoint` _asbp_race_kit_check_point)
        (:`>`
          (set `local.LocalResult` 1))
        (:`==`
          (set `local.LocalResult` 0))
        (:`<`
          (bind _output_get (set `local.LocalResult` -1)))))
    (:`CastFailed`
      _))
  (return _output_get))

(fn `GetCheckPointFront`
  (returns (ReturnValue :type "Vector Structure"))
  ;[1 1 1] Return the world space position of the front of the checkpoint.
  (return (`KismetMathLibrary.MakeVector` (- (.x (`self.K2_GetActorLocation`)) (.x (`BoxComponent.GetScaledBoxExtent` (`self.Box`)))) (.y (`self.K2_GetActorLocation`)) (.z (`self.K2_GetActorLocation`)))))

(fn `PlaceDebugActors`
  (bind _x (.x (`BoxComponent.BoxExtent` (`self.Box`))))
  (bind _z (.z (`BoxComponent.BoxExtent` (`self.Box`))))
  (`SceneComponent.K2_SetRelativeLocation` (`self. TextRender`) (`KismetMathLibrary.MakeVector` (+ (.x (`SceneComponent.RelativeLocation` (`self. TextRender`))) _x) 0.0 (- (.z (`SceneComponent.RelativeLocation` (`self. TextRender`))) _z)) false false)
  (`SceneComponent.K2_SetRelativeLocation` (`self.Arrow`) (`KismetMathLibrary.MakeVector` (+ _x (.x (`SceneComponent.RelativeLocation` (`self.Arrow`)))) 0.0 (- (.z (`SceneComponent.RelativeLocation` (`self.Arrow`))) _z)) false false))

(fn `SetBoxSize`
  ;[1 1 1] Set the size of the Checkpoint's box volume.
  (`BoxComponent.SetBoxExtent` (`self.Box`) (`self.CheckPointSize`) true))

(fn `SetDebugText`
  ;[1 1 1] If Debug is set to true, set a text render to the checkpoint number.
  (if (`self.DebugCheckPoint`)
    (`TextRenderComponent.K2_SetText` (`self. TextRender`) (`KismetTextLibrary.Conv_IntToText` (`self.CheckPoint`)))
    (else
      (`ActorComponent.SetActive` (`self. TextRender`) false false))))

(fn `UserConstructionScript`
  ;[1 1 1] Update checkpoint box volume size, place debug text render and arrow based on checkpoint volume size, and set the checkpoint number if debug flag is true.
  (`|ExecutionSequence`
    (:`then_0`
      (`self.SetBoxSize`))
    (:`then_1`
      (`self.PlaceDebugActors`))
    (:`then_2`
      (`self.SetDebugText`))))