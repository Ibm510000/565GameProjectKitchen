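; Race manager actor that runs one race, identified by RaceID, from optional countdown through timing, live positions and finish results.
; Construction gathers and sorts matching checkpoints and forces Lap mode for multi-lap races.
; Racer components register into a fixed slot array and a position array re-sorted every racing tick.
; Checkpoint queries resolve the next target, lap changes and finishes for Straight or Lap modes, optionally allowing shortcuts.
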(event `self.ReceiveBeginPlay`
  (`KismetSystemLibrary.Delay` 0.2)
  (`self.SortComponents`))

(event `self.ReceiveTick`
  (params (DeltaSeconds :type "Float (single-precision)"))
  (if (`self.Racing`)
    (`|ExecutionSequence`
      (:`then_0`
        (`self.SortComponents`))
      (:`then_1`
        (`self.CountRaceTime`)))))

(event `StartRace`
  (params (CountDown :type Boolean))
  (if CountDown
    (`self.StartRaceCountDown` (`self.RaceCountDownSeconds`))
    (else
      (`self.SetRaceStarted`))))

(event `RaceCountDownEvent`
  (params (TimeLeft :type Integer))
  (`self.RaceCountDown` TimeLeft))

(fn `CheckRaceFinished`
  (locals (LocalAllFinished :type Boolean :default true))
  ;[1 1 1] Race is finished when every registered component is not racing. If true, stop the race and call the RaceFinished event.
  (for _array_element (`self.RaceKitComponents`)
    (set `local.LocalAllFinished` (and (`local.LocalAllFinished`) (not (`/Game/RaceKit/Blueprints/BP_RaceKitComponent.Racing` _array_element)))))
  (if (`local.LocalAllFinished`)
    (set `self.Racing` false)
    (set `self.Finished` true)
    (`self.RaceFinished`)))

(fn `CompareCheckPoint`
  (params (HitCheckPoint :type Integer) (CurrentNextCheckPoint :type Integer) (Lap :type Integer))
  (returns (Finished :type Boolean))
  (locals (LocalHitCheckPoint :type Integer) (LocalLap :type Integer) (LocalNextCheckPoint :type Integer) (LocalCurrentNextCheckPoint :type Integer))
  (set `local.LocalHitCheckPoint` HitCheckPoint)
  (set `local.LocalCurrentNextCheckPoint` CurrentNextCheckPoint)
  (set `local.LocalLap` Lap)
  (switch `/Game/RaceKit/Blueprints/ERaceMode` (`self.RaceMode`)
    (:`NewEnumerator0`
      ;[1 1 1] Lap race is finished when last check point is hit.
      (return (== (- (`KismetArrayLibrary.Array_Length` (`self.CheckPoints`)) 1) (`local.LocalHitCheckPoint`))))
    (:`NewEnumerator1`
      ;[1 1 1] Lap race is finished when hitting the first check point on the final lap.
      (return (and (== (`local.LocalCurrentNextCheckPoint`) 0) (== 0 (`local.LocalHitCheckPoint`)) (== (`local.LocalLap`) (`self.Laps`)))))))

(fn `CountRaceTime`
  ;[1 1 1] Count the time elapsed of the current race.
  (set `self.RaceTime` (+ (`self.RaceTime`) (`GameplayStatics.GetWorldDeltaSeconds`)))
  (return))

(fn `FindCheckPoints`
  ;[1 1 1] Find all checkpoints in the map.
  (`KismetArrayLibrary.Array_Clear` (`self.CheckPoints`))
  (bind _outactors (`GameplayStatics.GetAllActorsOfClass` "/Game/RaceKit/Blueprints/BP_RaceKitCheckPoint.BP_RaceKitCheckPoint_C"))
  ;[1 1 1] Save if RaceID matches that of this race.
  (for _array_element _outactors
    (if (== (`/Game/RaceKit/Blueprints/BP_RaceKitCheckPoint.RaceID` _array_element) (`self.RaceID`))
      (`KismetArrayLibrary.Array_Add` (`self.CheckPoints`) _array_element)))
  ;[1 1 1] Sort into order.
  (`/Game/RaceKit/Blueprints/BPFL_RaceKitFunctions.Sort` (`self.CheckPoints`)))

(fn `FinishedRacer`
  (params (RacerSlot :type Integer))
  (bind _racekitcomponent (`self.GetRacer` RacerSlot))
  ;[1 1 1] When racer finishes, add relevant data to Finished Racer struct and add to finished race array.
  (bind _returnvalue (`KismetArrayLibrary.Array_Add` (`self.FinishedRace`) (make `/Game/RaceKit/Blueprints/SFinishedRacer` RacerSlot (`/Game/RaceKit/Blueprints/BP_RaceKitComponent.BestLapTime` _racekitcomponent) (`self.RaceTime`))))
  ;[1 1 1] Set the finished racer component's position and finished bool, check if all racers are finished.
  (set `/Game/RaceKit/Blueprints/BP_RaceKitComponent.FinishedPosition` _returnvalue _racekitcomponent)
  (set `/Game/RaceKit/Blueprints/BP_RaceKitComponent.Finished` true _racekitcomponent)
  (`self.CheckRaceFinished`))

(fn `GetCheckPoint`
  (params (HitCheckPoint :type Integer) (CurrentNextCheckPoint :type Integer))
  (returns (RaceKitCheckPoint :type "/Game/RaceKit/Blueprints/BP_RaceKitCheckPoint Object Reference") (NextCheckPoint :type Integer) (NextLap :type Boolean))
  (locals (LocalNextCheckPoint :type Integer) (LocalCurrentNextCheckPoint :type Integer))
  (bind _localcurrentnextcheckpoint (`local.LocalCurrentNextCheckPoint`))
  ;[1 1 1] Save variables and switch on RaceMode
  (set `local.LocalNextCheckPoint` (+ HitCheckPoint 1))
  (set `local.LocalCurrentNextCheckPoint` CurrentNextCheckPoint)
  (if (`self.AllowShortcuts`)
    _
    (elif (== (- (`local.LocalNextCheckPoint`) 1) (`local.LocalCurrentNextCheckPoint`))
      _
      (else
        ;[1 1 1] If not allowing shortcuts, bail out if hit checkpoint isn't the next checkpoint
        (return (`|GetArrayItem` (`self.CheckPoints`) _localcurrentnextcheckpoint) _localcurrentnextcheckpoint false))))
  (switch `/Game/RaceKit/Blueprints/ERaceMode` (`self.RaceMode`)
    (:`NewEnumerator0`
      ;[1 1 1] Check for last check point hit.
      (if (== (`local.LocalNextCheckPoint`) (`KismetArrayLibrary.Array_Length` (`self.CheckPoints`)))
        ;[1 1 1] Return first check point.
        (return (`|GetArrayItem` (`self.CheckPoints`)) 0 true)
        (else
          ;[1 1 1] Return next check point.
          (return (`|GetArrayItem` (`self.CheckPoints`) (`local.LocalNextCheckPoint`)) (`local.LocalNextCheckPoint`) false))))
    (:`NewEnumerator1`
      ;[1 1 1] Check for last check point hit.
      (if (== (`local.LocalNextCheckPoint`) (`KismetArrayLibrary.Array_Length` (`self.CheckPoints`)))
        ;[1 1 1] Return first check point.
        (return (`|GetArrayItem` (`self.CheckPoints`)) 0 false)
        (else
          ;[1 1 1] Check if supposed to be hitting finish check point next, for next lap.
          (if (and (== (`local.LocalCurrentNextCheckPoint`) 0) (== (- (`local.LocalNextCheckPoint`) 1) 0))
            ;[1 1 1] Return first check point, toggle next lap.
            (return (`|GetArrayItem` (`self.CheckPoints`) (`local.LocalNextCheckPoint`)) (`local.LocalNextCheckPoint`) true)
            (else
              ;[1 1 1] Return next check point.
              (return (`|GetArrayItem` (`self.CheckPoints`) (`local.LocalNextCheckPoint`)) (`local.LocalNextCheckPoint`) false))))))))

(fn `GetFinishedRaceData`
  (returns (RaceID :type Integer) (RaceTime :type "Float (double-precision)") (FinishedRace :type "Array of /Game/RaceKit/Blueprints/SFinishedRacer Structure"))
  ;[1 1 1] Return finished race data for this race.
  (return (`self.RaceID`) (`self.RaceTime`) (`self.FinishedRace`)))

(fn `GetPlayerLastCheckpoint`
  (params (Controller :type "PlayerController Object Reference"))
  (returns (Checkpoint :type "/Game/RaceKit/Blueprints/BP_RaceKitCheckPoint Object Reference"))
  (bind _returnvalue (`self.GetComponentByClass` (`Controller.K2_GetPawn` Controller) "/Game/RaceKit/Blueprints/BP_RaceKitComponent.BP_RaceKitComponent_C"))
  (if (`KismetSystemLibrary.IsValid` _returnvalue)
    (return (`|GetArrayItem` (`self.CheckPoints`) (- (`.NextCheckPoint` (`/Game/RaceKit/Blueprints/BP_RaceKitComponent.GetData` _returnvalue)) 1)))))

(fn `GetRacer`
  (params (Slot :type Integer))
  (returns (RaceKitComponent :type "/Game/RaceKit/Blueprints/BP_RaceKitComponent Object Reference"))
  ;[1 1 1] Get Race Kit Component from slotted component array.
  (return (`|GetArrayItem` (`self.SlottedRaceKitComponents`) Slot)))

(fn `RegisterRacer`
  (params (RaceKitComponent :type "/Game/RaceKit/Blueprints/BP_RaceKitComponent Object Reference"))
  ;[1 1 1] Add into an array of slotted components for easy retrieval.
  (`KismetArrayLibrary.Array_Add` (`self.SlottedRaceKitComponents`) RaceKitComponent)
  ;[1 1 1] Add into an array that will be sorted on position and set the slot on the registered component.
  (bind _returnvalue (`KismetArrayLibrary.Array_Add` (`self.RaceKitComponents`) RaceKitComponent))
  (set `/Game/RaceKit/Blueprints/BP_RaceKitComponent.RacerSlot` _returnvalue RaceKitComponent))

(fn `ResetRace`
  ;[1 1 1] Reset race data for a new race. Save finished race data before calling this, if needed.
  (`KismetArrayLibrary.Array_Clear` (`self.RaceKitComponents`))
  (`KismetArrayLibrary.Array_Clear` (`self.SlottedRaceKitComponents`))
  (set `self.RaceTime` 0.0)
  (`KismetArrayLibrary.Array_Clear` (`self.FinishedRace`)))

(fn `SetRaceMode`
  (if (> (`self.Laps`) 1)
    (if (`|EnumEquality` (`self.RaceMode`) "NewEnumerator0")
      (set `self.RaceMode` "NewEnumerator1"))))

(fn `SetRaceStarted`
  ;[1 1 1] Set race started on this manager and all registered components, call race started event.
  (set `self.Racing` true)
  (for _array_element (`self.RaceKitComponents`)
    (set `/Game/RaceKit/Blueprints/BP_RaceKitComponent.Racing` true _array_element))
  (`self.RaceStarted`))

(fn `SortComponents`
  (if (> (`KismetArrayLibrary.Array_Length` (`self.RaceKitComponents`)) 1)
    (`/Game/RaceKit/Blueprints/BPFL_RaceKitFunctions.Sort` (`self.RaceKitComponents`))
    (for (_array_element _array_index) (`self.RaceKitComponents`)
      (set `/Game/RaceKit/Blueprints/BP_RaceKitComponent.Position` _array_index _array_element))))

(fn `UserConstructionScript`
  (`self.FindCheckPoints`)
  (`self.SetRaceMode`))