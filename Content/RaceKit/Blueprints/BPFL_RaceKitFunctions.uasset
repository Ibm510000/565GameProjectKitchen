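; Blueprint function library for the Race Kit, providing manager lookup and generic object sorting.
; GetRaceKitManager searches all BP_RaceKitManager actors in the map and returns the one with the matching RaceID.
; Sort runs an early-exit bubble sort in either direction, ordering objects through a CompareTo interface message, then writes the result back to the by-ref input array and also returns it.
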(fn GetRaceKitManager
  (params (RaceID :type Integer))
  ;[1 1 1] Return the Race Kit Manager in the map of the desired RaceID.
  (bind _outactors (Actor|GetAllActorsOfClass 0 "/Game/RaceKit/Blueprints/BP_RaceKitManager.BP_RaceKitManager_C"))
  (for _array_element _outactors
    (if (== (Variables|/Game/RaceKit/Blueprints/BP_RaceKitManager.BP_RaceKitManager_C|GetRaceID _array_element) RaceID)
      (return _array_element))))

(fn Sort
  (params (Objects :type Array%20of%20Object%20Object%20References) (Ascending :type Boolean))
  ;[1 1 1] Bubble sort blueprint array implementation
  ;[1 1 1] Set direction of sort and local copy of input array.
  (if Ascending
    (LocalVariables|SetSortDirection 1)
    (else
      (LocalVariables|SetSortDirection -1)))
  (LocalVariables|SetLocalObjects Objects)
  ;[1 1 1] For each index of the array, while no swaps are needed
  (while (LocalVariables|GetLocalSwapped)
    (LocalVariables|SetLocalSwapped false)
    (Math|Integer|IncrementInt (LocalVariables|GetLocalSortIndex)
      (:%20%20
        (for _index (range 0 (- (- (Utilities|Array|Length (LocalVariables|GetLocalObjects)) (LocalVariables|GetLocalSortIndex)) 1))
          ;[1 1 1] Compare the objects using the Compare To interface
          (bind _result (Class|BPISortInterface|Compareto(Message) (Utilities|Array|Get(acopy) (LocalVariables|GetLocalObjects) _index) (Utilities|Array|Get(acopy) (LocalVariables|GetLocalObjects) (+ _index 1))))
          ;[1 1 1] Swap if out of order
          (if (== _result (LocalVariables|GetSortDirection))
            (LocalVariables|SetLocalSortObject (Utilities|Array|Get(acopy) (LocalVariables|GetLocalObjects) _index))
            (Utilities|Array|SetArrayElem (LocalVariables|GetLocalObjects) _index (Utilities|Array|Get(acopy) (LocalVariables|GetLocalObjects) (+ _index 1)))
            (Utilities|Array|SetArrayElem (LocalVariables|GetLocalObjects) (+ _index 1) (LocalVariables|GetLocalSortObject))
            (LocalVariables|SetLocalSwapped true))))))
  ;[1 1 1] Set the input array into the sorted array, return sorted array.
  (|SetBy-RefVar Objects (LocalVariables|GetLocalObjects))
  (return (LocalVariables|GetLocalObjects)))