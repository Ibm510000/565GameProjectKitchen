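; BP_Stove is a kitchen stove prop with adjustable top and bottom doors, posed entirely in the Construction Script with no active runtime logic.
; Open/close values are lerped into roll rotations on each door's pivot, and a flag shows or hides the top door mesh.
; Three lights become visible once the bottom door's open value passes a threshold.
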(fn `UserConstructionScript`
  (`|ExecutionSequence`
    (:`then_0`
      (`SceneComponent.SetVisibility` (`self.SM_StoveTopDoor`) (`self.Top door visible`) false)
      (`SceneComponent.K2_SetRelativeRotation` (`self.TopDoorPivot`) (`KismetMathLibrary.MakeRotator` (* (`KismetMathLibrary.Lerp` 0.0 240.0 (`self.Open / Close Top Door`)) -1.0)) false false))
    (:`then_1`
      (`SceneComponent.K2_SetRelativeRotation` (`self.DownDoorPivot`) (`KismetMathLibrary.MakeRotator` (`KismetMathLibrary.Lerp` 0.0 90.0 (`self.Open / Close Bottom Door`))) false false)
      (`SceneComponent.SetVisibility` (`self.Light1`) (> (`self.Open / Close Bottom Door`) 0.4) false)
      (`SceneComponent.SetVisibility` (`self.Light2`) (> (`self.Open / Close Bottom Door`) 0.4) false)
      (`SceneComponent.SetVisibility` (`self.Light3`) (> (`self.Open / Close Bottom Door`) 0.4) false))))