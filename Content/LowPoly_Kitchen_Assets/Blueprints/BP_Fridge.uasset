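; BP_Fridge is a kitchen fridge prop with top and down doors, each posed by its own open/close value.
; The construction script lerps each value into a yaw rotation on that door's pivot, swinging it up to 170 degrees in the negative direction.
; Each door's light becomes visible once its value passes a small threshold.
; The event graph is empty, so doors and lights only update when construction runs.
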(event `self.ReceiveBeginPlay`)

(fn `UserConstructionScript`
  (`|ExecutionSequence`
    (:`then_0`
      (`SceneComponent.K2_SetRelativeRotation` (`self.TopDoorPivot`) (`KismetMathLibrary.MakeRotator` 0.0 0.0 (* (`KismetMathLibrary.Lerp` 0.0 170.0 (`self.Open / Close Top  Door`)) -1.0)) false false)
      (`SceneComponent.SetVisibility` (`self.Light1`) (> (`self.Open / Close Top  Door`) 0.1) false))
    (:`then_1`
      (`SceneComponent.K2_SetRelativeRotation` (`self.DownDoorPivot`) (`KismetMathLibrary.MakeRotator` 0.0 0.0 (* (`KismetMathLibrary.Lerp` 0.0 170.0 (`self.Open / Close Down Door`)) -1.0)) false false)
      (`SceneComponent.SetVisibility` (`self.Light2`) (> (`self.Open / Close Down Door`) 0.1) false))))