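; Player pawn that rolls a physics sphere along the camera's forward direction.
; Move adds input to an accumulated force, which Tick applies to the sphere as an acceleration with a red debug line, then decays toward zero via FInterpTo.
; Tick also moves the spring arm to the sphere's location without changing its rotation; velocity-based arm rotation logic is left unconnected.
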(event `self.ReceiveTick`
  (params (DeltaSeconds :type "Float (single-precision)"))
  (bind _curforce (`self.CurForce`))
  (`|ExecutionSequence`
    (:`then_0`
      (`self.ApplyForce` _curforce)
      (set `self.CurForce` (`KismetMathLibrary.FInterpTo` _curforce 0.0 DeltaSeconds (`self.ForceDecayRate`))))
    (:`then_1`
      (`SceneComponent.K2_SetWorldLocation` (`self.SpringArm`) (`SceneComponent.K2_GetComponentLocation` (`self.Sphere`)) false false))))

(fn `ApplyForce`
  (params (Input :type "Float (double-precision)"))
  (bind _returnvalue (`SceneComponent.K2_GetComponentLocation` (`self.Sphere`)))
  (bind _forward (`self.GetBallMoveSpace`))
  (bind _returnvalue_2 (* _forward Input))
  (`PrimitiveComponent.AddForce` (`self.Sphere`) _returnvalue_2 "None" true)
  (`KismetSystemLibrary.DrawDebugLine` _returnvalue (+ _returnvalue _returnvalue_2) (struct :`R` 1.0 :`A` 1.0)))

(fn `GetBallMoveSpace`
  (returns (Forward :type "Vector Structure") (Right :type "Vector Structure"))
  (bind _camrotation (`self.CamRotation`))
  (return (`SceneComponent.GetForwardVector` _camrotation) (`SceneComponent.GetRightVector` _camrotation)))

(fn `Move`
  (params (Input :type "Float (double-precision)"))
  (set `self.CurForce` (+ (`self.CurForce`) Input)))

(fn `UserConstructionScript`)