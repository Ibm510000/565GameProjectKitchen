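; AI controller that drives a possessed BP_AIPawn toward its next race checkpoint.
; Every tick it finds a navmesh path to the ground point of the checkpoint indexed by the pawn's race kit component.
; It pushes the pawn along the first path segment with a scaled unit-direction force.
; Without a usable path, it heads for a random reachable nearby point, then a projected navmesh point, else prints an error.
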(event `self.ReceiveTick`
  (params (DeltaSeconds :type "Float (single-precision)"))
  (`self.GetNextPath`))

(event `self.ReceivePossess`
  (params (PossessedPawn :type "Pawn Object Reference"))
  (bind _asbp_aipawn (cast `/Game/OurGame/BP/BP_AIPawn` PossessedPawn))
  (set `self.AIPawn` _asbp_aipawn))

(fn `GetNextPath`
  (locals (NoPath :type Boolean))
  (bind _aipawn (`self.AIPawn`))
  (bind _worldloc (`/Game/OurGame/BP/BP_AIPawn.GetLocation` (`self.AIPawn`)))
  (bind _worldloc_2 (`/Game/OurGame/BP/BP_AIPawn.GetLocation` (`self.AIPawn`)))
  (if (`KismetSystemLibrary.IsValid` (`self.AIPawn`))
    (bind _racekitmanager (`/Game/RaceKit/Blueprints/BPFL_RaceKitFunctions.GetRaceKitManager` 0))
    (bind _returnvalue (`/Game/RaceKit/Blueprints/BP_RaceKitCheckPoint.Get Ground Point` (`|GetArrayItem` (`/Game/RaceKit/Blueprints/BP_RaceKitManager.CheckPoints` _racekitmanager) (`/Game/RaceKit/Blueprints/BP_RaceKitComponent.NextCheckPoint` (`/Game/OurGame/BP/BP_AIPawn.BP_RaceKitComponent` (`self.AIPawn`))))))
    (bind _returnvalue_2 (`NavigationSystemV1.FindPathToLocationSynchronously` (`/Game/OurGame/BP/BP_AIPawn.GetLocation` _aipawn) _returnvalue _aipawn null))
    (bind _pathpoints (`NavigationPath.PathPoints` _returnvalue_2))
    (if (< (`KismetArrayLibrary.Array_Length` _pathpoints) 2)
      (bind _returnvalue_3 (`GameplayStatics.GetActorOfClass` "/Script/NavigationSystem.RecastNavMesh"))
      (bind (_randomlocation _returnvalue_4) (`NavigationSystemV1.K2_GetRandomReachablePointInRadius` _worldloc_2 1000.0 _returnvalue_3 null))
      (if _returnvalue_4
        (`self.GoTo` _worldloc_2 _randomlocation)
        (else
          (bind (_projectedlocation _returnvalue_5) (`NavigationSystemV1.K2_ProjectPointToNavigation` _worldloc _returnvalue_3 null (1000.0 1000.0 0.0)))
          (if _returnvalue_5
            (`self.GoTo` _worldloc _projectedlocation)
            (else
              (`KismetSystemLibrary.PrintString` "No Path!!")))))
      (else
        (`self.GoTo` (`|GetArrayItem` _pathpoints) (`|GetArrayItem` _pathpoints 1))))))

(fn `UserConstructionScript`)