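; AI-driven ball pawn for races that spawns and is possessed by its own BP_AIBallController at BeginPlay.
; It binds to the race kit manager's race-started event to enable control.
; AddForce applies velocity-change impulses to the Sphere while control is enabled, and GetLocation returns the Sphere's position.
; ClearForce only toggles the control flag, as the physics-simulation switch in SetCanControl is disconnected.
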(event `self.ReceiveBeginPlay`
  (bind _racekitmanager (`/Game/RaceKit/Blueprints/BPFL_RaceKitFunctions.GetRaceKitManager` 0))
  (add `/Game/RaceKit/Blueprints/BP_RaceKitManager.RaceStarted` _racekitmanager (`|CreateDelegate` :!event `RaceStarted`))
  (bind _returnvalue (`|SpawnActorFromClass` "/Game/OurGame/BP/BP_AIBallController.BP_AIBallController_C" (`self.GetTransform`) "Undefined" "MultiplyWithRoot" null null))
  (`Controller.Possess` _returnvalue self))

(event `self.ReceiveTick`
  (params (DeltaSeconds :type "Float (single-precision)")))

(fn `AddForce`
  (params (Input :type "Vector Structure"))
  (if (`self.CanControl`)
    (`PrimitiveComponent.AddImpulse` (`self.Sphere`) Input "None" true)))

(fn `ClearForce`
  (if (`self.CanControl`)
    (`self.SetCanControl` false)
    (`self.SetCanControl` true)))

(fn `GetLocation`
  (returns (worldLoc :type "Vector Structure"))
  (return (`SceneComponent.K2_GetComponentLocation` (`self.Sphere`))))

(fn `RaceStarted`
  (`self.SetCanControl` true))

(fn `SetCanControl`
  (params (CanControl :type Boolean))
  (bind _output_get (set `self.CanControl` CanControl)))

(fn `UserConstructionScript`)