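; Soviet kitchen furniture prop with four drawers and two upper rotating parts, likely doors, that can be posed per instance.
; The construction script shifts each drawer by its own local offset variable and rotates UpLeft and UpRight by their rotation variables.
; It has no runtime logic, as the event graph holds only disabled default events.
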(fn `UserConstructionScript`
  (`SceneComponent.K2_AddLocalOffset` (`self.Drawer01`) (`self.Drawer1`) false false)
  (`SceneComponent.K2_AddLocalOffset` (`self.Drawer02`) (`self.Drawer2`) false false)
  (`SceneComponent.K2_AddLocalOffset` (`self.Drawer03`) (`self.Drawer3`) false false)
  (`SceneComponent.K2_AddLocalOffset` (`self.Drawer04`) (`self.Drawer4`) false false)
  (`SceneComponent.K2_AddLocalRotation` (`self.UpLeft`) (`self.Up_Left`) false false)
  (`SceneComponent.K2_AddLocalRotation` (`self.UpRight`) (`self.Up_Right`) false false))