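; BP_Window01 is a window Blueprint in the SovietKitchen content whose glass and add-on components can be posed through rotation values.
; The Construction Script adds local rotations to three glass and add-on pairs: the first uses Add01, the second and third share Add02.
; The third pair also receives Add03 on top of Add02.
; The Event Graph holds only disabled default events, so it has no runtime logic.
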(fn `UserConstructionScript`
  (`SceneComponent.K2_AddLocalRotation` (`self.Window_glass_01`) (`self.Add_01`) false false)
  (`SceneComponent.K2_AddLocalRotation` (`self.Window_add_01`) (`self.Add_01`) false false)
  (`SceneComponent.K2_AddLocalRotation` (`self.Window_add_02`) (`self.Add_02`) false false)
  (`SceneComponent.K2_AddLocalRotation` (`self.Window_glass_02`) (`self.Add_02`) false false)
  (`SceneComponent.K2_AddLocalRotation` (`self.Window_add_03`) (`self.Add_02`) false false)
  (`SceneComponent.K2_AddLocalRotation` (`self.Window_glass_03`) (`self.Add_02`) false false)
  (`SceneComponent.K2_AddLocalRotation` (`self.Window_add_03`) (`self.Add_03`) false false)
  (`SceneComponent.K2_AddLocalRotation` (`self.Window_glass_03`) (`self.Add_03`) false false))