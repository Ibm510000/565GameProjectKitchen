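; Kitchen furniture actor for the Soviet Kitchen set, with four separately rotatable parts named by position: upper and lower, left and right.
; The construction script adds a local rotation to each part from its matching variable, so the pose is set at construction time.
; The event graph holds only empty default events, so the Blueprint adds no runtime behavior.
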(fn `UserConstructionScript`
  (`SceneComponent.K2_AddLocalRotation` (`self.Up_Left`) (`self.UpLeft`) false false)
  (`SceneComponent.K2_AddLocalRotation` (`self.Up_Right`) (`self.UpRight`) false false)
  (`SceneComponent.K2_AddLocalRotation` (`self.Down_Left`) (`self.DownLeft`) false false)
  (`SceneComponent.K2_AddLocalRotation` (`self.Down_Right`) (`self.DownRight`) false false))